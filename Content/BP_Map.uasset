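; Map actor that builds a tile-based level from a data table when play begins.
; It reads each row's X, Y, Height and Type, then spawns a BP_Tile at a grid position relative to itself, scaled by TileDistance.
; Height steps are one third of the tile spacing, and the integer Type is converted to a tile type and applied to each spawned tile.
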(event EventBeginPlay
  (bind _tiledistance (Variables|Default|GetTileDistance))
  (bind _outrownames (DataTable|GetDataTableRowNames "/Game/map.map"))
  (for _array_element _outrownames
    (bind _returnvalue (Utilities|GetDataTableRow "/Game/map.map" _array_element)
      (:then
        (bind _returnvalue_2 (Game|SpawnActorfromClass "/Game/BP_Tile.BP_Tile_C" (Math|Conversions|ToTransform(Vector) (+ (Math|Vector|MakeVector (Math|Conversions|ToFloat(Integer) (* (.x (Utilities|Struct|BreakTileStruct _returnvalue)) _tiledistance)) (Math|Conversions|ToFloat(Integer) (* _tiledistance (.y (Utilities|Struct|BreakTileStruct _returnvalue)))) (Math|Conversions|ToFloat(Integer) (* (/ _tiledistance 3) (.height (Utilities|Struct|BreakTileStruct _returnvalue))))) (Transformation|GetActorLocation))) "AlwaysSpawn" self 0))
        (bind _tiletype (CallFunction|GetTileTypefromInt (.type (Utilities|Struct|BreakTileStruct _returnvalue))))
        (Default|SetType _returnvalue_2 _tiletype)))))

(fn ConstructionScript)